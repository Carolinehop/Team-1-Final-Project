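; Wall-or-world button Blueprint with a light bulb material that activates its selected doors once when E is pressed inside its trigger.
; Trigger overlap enables input and opens a gate; leaving disables input and switches the light off.
; A press lights the bulb via a dynamic material instance, calls ActivateDoor if the overlapping actor is a Character, then sets OnOff to block further presses.
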(event `Key|E`
  (params (Key :type "Key Structure" :default "AnyKey"))
  (bind _selecteddoor (`self.SelectedDoor`))
  (:`Pressed`
    (if (not (`self.On/Off`))
      (`/Engine/EditorBlueprintResources/StandardMacros.Gate` true :!label _label
        (:`Exit`
          (`|ExecutionSequence`
            (:`then_0`
              (`MaterialInstanceDynamic.SetScalarParameterValue` (`self.Button light material`) "State" 1.0))
            (:`then_1`
              (cast `Character` (stale `self.Trigger collision.OnComponentBeginOverlap` OtherActor))
              (for _ _selecteddoor
                (`/Game/ExampleContent/Blueprints/Blueprints/BP_Door.Activate Door` _selecteddoor)))
            (:`then_2`
              (set `self.On/Off` true))))))))

(event `self.Trigger collision.OnComponentBeginOverlap`
  (params (OverlappedComponent :type "PrimitiveComponent Object Reference") (OtherActor :type "Actor Object Reference") (OtherComp :type "PrimitiveComponent Object Reference") (OtherBodyIndex :type Integer) (bFromSweep :type Boolean) (SweepResult :type "HitResult Structure (by ref)"))
  (`self.EnableInput` (`GameplayStatics.GetPlayerController` 0))
  (goto _label :!via `Open`))

(event `self.Trigger collision.OnComponentEndOverlap`
  (params (OverlappedComponent :type "PrimitiveComponent Object Reference") (OtherActor :type "Actor Object Reference") (OtherComp :type "PrimitiveComponent Object Reference") (OtherBodyIndex :type Integer))
  (`self.DisableInput` (`GameplayStatics.GetPlayerController` 0))
  (`MaterialInstanceDynamic.SetScalarParameterValue` (`self.Button light material`) "State" 0.0))

(fn `UserConstructionScript`
  (bind _returnvalue (`PrimitiveComponent.CreateDynamicMaterialInstance` (`self.ButtonMesh`) 2 null))
  (set `self.Button light material` _returnvalue) ; Save a reference to the Dynamic Material Instance for use in the event graph
  (set `self.On/Off` false))